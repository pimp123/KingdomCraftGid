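; Main menu game mode that sets up each new player's menu view, saved character and HUD, and launches the selected level.
; On player start it has BP_PC_MainMenu set the camera target and spawn the saved character, then creates WBP_MainMenu with UI-only input.
; The default row of the D_Maps data table seeds MapInformation, which feeds the widget's map info panel and supplies the level name LaunchLevel opens.
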(event `self.HandleStartingNewPlayer`
  (params (NewPlayer :type "PlayerController Object Reference"))
  ;[1 1 1] starting new player, update camera view, spawn character and create HUD
  (bind _asbp_pc_main_menu (cast `/Game/Asset/SingleplayerMenu/Blueprints/Controllers/BP_PC_MainMenu` NewPlayer))
  (`/Game/Asset/SingleplayerMenu/Blueprints/Controllers/BP_PC_MainMenu.SetNewViewTargetForPlayer` _asbp_pc_main_menu)
  (`/Game/Asset/SingleplayerMenu/Blueprints/Controllers/BP_PC_MainMenu.SpawnMainMenuCharacter` _asbp_pc_main_menu (`/Game/Asset/SingleplayerMenu/Blueprints/FunctionLibraries/BFL_All.GetUserSavedCharacter`))
  (`self.CreateMainMenuHUD`)
  (`self.SetDefaultLevel`))

(event `SetDefaultLevel`
  ;[1 1 1] set default level
  (bind _returnvalue (`|GetDataTableRow` "/Game/Asset/SingleplayerMenu/Datatables/D_Maps.D_Maps" "Default")
    (:`then`
      (`self.UpdateLevelInformation` _returnvalue))))

(event `UpdateLevelInformation`
  (params (S_Maps :type "/Game/Asset/SingleplayerMenu/Structures/S_Maps Structure"))
  ;[1 1 1] update level information
  (bind _output_get (set `self.MapInformation` S_Maps))
  (bind _wbp_mainmenu (`self.WBP_MainMenu`)
    (:`then`
      (`/Game/Asset/SingleplayerMenu/Widgets/WBP_LevelInformation.UpdateLevelInformationOnWidget` (`/Game/Asset/SingleplayerMenu/Widgets/WBP_MainMenu.WBP_MapInfo` _wbp_mainmenu) _output_get))
    (:`else`)))

(event `CreateMainMenuHUD`
  ;[1 1 1] create main menu widget on client
  (bind _returnvalue (`|CreateWidget` "/Game/Asset/SingleplayerMenu/Widgets/WBP_MainMenu.WBP_MainMenu_C"))
  (bind _output_get (set `self.WBP_MainMenu` _returnvalue))
  (`UserWidget.AddToViewport` _output_get 0)
  (`WidgetBlueprintLibrary.SetInputMode_UIOnlyEx` (`GameplayStatics.GetPlayerController` 0) _returnvalue))

(event `LaunchLevel`
  ;[1 1 1] launch level
  (`GameplayStatics.OpenLevel` (`.LevelName_14_ABE1869A49AC3B78614CF6BBD72FF46E` (break `/Game/Asset/SingleplayerMenu/Structures/S_Maps` (`self.MapInformation`)))))

(fn `UserConstructionScript`)