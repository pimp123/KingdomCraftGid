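; Base physics-driven player that walks and moves through the air under arbitrary gravity directions.
; Each tick, a sphere trace with line-trace fallback finds walkable ground, switching damping and camera-relative forces between ground and air.
; Ground movement follows the surface plane and compensates for gravity along slopes.
; The standing axis turns against GravityReceiver's accumulated gravity at a limited rate, rotating the capsule and optionally preserving the camera's look direction.
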(event `self.ReceiveTick`
  (params (DeltaSeconds :type "Float (single-precision)"))
  (bind _groundaxis (`self.GroundAxis`))
  (bind _cameraholder (`self.CameraHolder`))
  (bind _cameraholder_2 (`self.CameraHolder`))
  (bind _returnvalue (* DeltaSeconds (`self.StandingTurnRate`)))
  (bind _gravityaccumulator (`/Game/Asset/DirectionalGravity/Blueprints/GravityLogic/BP_GravityReceiver.GravityAccumulator` (`self.GravityReceiver`)))
  (bind _movementdirection (`self.CalculateMovementDirection` (`SceneComponent.GetForwardVector` _cameraholder) (`SceneComponent.GetRightVector` _cameraholder)))
  (bind _movementdirection_2 (`self.CalculateMovementDirection` (`self.CorrectMovementDirection` (`SceneComponent.GetForwardVector` _cameraholder_2) _groundaxis) (`self.CorrectMovementDirection` (`SceneComponent.GetRightVector` _cameraholder_2) _groundaxis)))
  (bind _returnvalue_2 (* (`KismetMathLibrary.Normal` _gravityaccumulator) -1.0))
  (bind (_axis _angle) (`/Game/Asset/DirectionalGravity/Blueprints/Helpers/BP_MathHelpers.AxisAngleBetween` (`self.StandingAxis`) _returnvalue_2))
  (bind _returnvalue_3 (`KismetMathLibrary.Abs` _angle))
  (`self.CheckIsOnGround`)
  (`PrimitiveComponent.SetLinearDamping` (`self.WalkCollision`) (`KismetMathLibrary.SelectFloat` (`self.GroundDamping`) (`self.AirDamping`) (`self.IsOnGround`)))
  (`|ExecutionSequence`
    (:`then_0`
      ;[1 1 1] Movement
      (if (or (!= (`self.ForwardDeltaMove`) 0.0) (!= (`self.RightDelataMove`) 0.0))
        (`self.CE_GetMove` true)
        (if (`self.IsOnGround`)
          ;;[1 1 1] Ground movement
          (set `self.MovementDirection` _movementdirection_2)
          (`PrimitiveComponent.AddForce` (`self.WalkCollision`) (* _movementdirection_2 (- (`self.WalkAcceleration`) (`KismetMathLibrary.Dot_VectorVector` (`/Game/Asset/DirectionalGravity/Blueprints/GravityLogic/BP_GravityReceiver.GravityAccumulator` (`self.GravityReceiver`)) _movementdirection_2))) "None" true)
          (else
            ;;[1 1 1] Air movement
            (set `self.MovementDirection` _movementdirection)
            (`PrimitiveComponent.AddForce` (`self.WalkCollision`) (* _movementdirection (`self.FlyAcceleration`)) "None" true)))
        (set `self.ForwardDeltaMove` 0.0)
        (set `self.RightDelataMove` 0.0)
        (else
          (set `self.MovementDirection` (0.0 0.0 0.0))
          (`self.CE_GetMove` false))))
    (:`then_1`
      ;[1 1 1] Orient player
      (if (!= _gravityaccumulator (0.0 0.0 0.0))
        (if (not (`KismetMathLibrary.NearlyEqual_FloatFloat` (`KismetMathLibrary.Dot_VectorVector` _returnvalue_2 (`self.StandingAxis`)) 1.0))
          (if (< _returnvalue_3 (`self.MinStandingTurnAngle`))
            (set `self.StandingAxis` _returnvalue_2)
            (elif (>= _returnvalue _returnvalue_3)
              (set `self.StandingAxis` (`KismetMathLibrary.Normal` (`KismetMathLibrary.RotateAngleAxis` (`self.StandingAxis`) _angle _axis)))
              (else
                (set `self.StandingAxis` (`KismetMathLibrary.Normal` (`KismetMathLibrary.RotateAngleAxis` (`self.StandingAxis`) (* _returnvalue (`KismetMathLibrary.SelectFloat` 1.0 -1.0 (> _angle 0.0))) _axis))))))
          (`self.UpdateStanding`))))))

(event `CE_GetMove`
  (params (IsMove :type Boolean)))

(fn `CalculateMovementDirection`
  (params (Forward :type "Vector Structure") (Right :type "Vector Structure"))
  (returns (MovementDirection :type "Vector Structure"))
  (return (`KismetMathLibrary.Normal` (+ (* Forward (`self.ForwardDeltaMove`)) (* Right (`self.RightDelataMove`))))))

(fn `CheckIsOnGround`
  (bind _array (`|MakeArray` "ObjectTypeQuery1" "ObjectTypeQuery4" "ObjectTypeQuery5" "ObjectTypeQuery2" :!type "EObjectTypeQuery Enum"))
  (bind _standingaxis (`self.StandingAxis`))
  (bind _groundsensitivity (`self.GroundSensitivity`))
  (bind _walkcollision (`self.WalkCollision`))
  (bind _returnvalue (`CapsuleComponent.GetScaledCapsuleRadius` _walkcollision))
  (bind _returnvalue_2 (* _returnvalue 1.5))
  (bind _returnvalue_3 (- (`SceneComponent.K2_GetComponentLocation` _walkcollision) (* _standingaxis (- (`CapsuleComponent.GetScaledCapsuleHalfHeight` _walkcollision) _returnvalue_2))))
  (bind (_outhit _returnvalue_4) (`KismetSystemLibrary.SphereTraceSingleForObjects` _returnvalue_3 (- _returnvalue_3 (* _standingaxis (+ (* _returnvalue 0.5) _groundsensitivity))) _returnvalue _array))
  (if (not _returnvalue_4)
    (set `self.IsOnGround` false)
    (else
      (bind _returnvalue_5 (`KismetMathLibrary.Normal` (`.ImpactNormal` (`GameplayStatics.BreakHitResult` _outhit))))
      (if (<= (`/Game/Asset/DirectionalGravity/Blueprints/Helpers/BP_MathHelpers.AngleBetween` _returnvalue_5 (`self.StandingAxis`)) (`self.GroundMaxSlopeAngle`))
        (set `self.GroundAxis` _returnvalue_5)
        (set `self.IsOnGround` true)
        (else
          (bind (_outhit_2 _returnvalue_6) (`KismetSystemLibrary.LineTraceSingleForObjects` _returnvalue_3 (- _returnvalue_3 (* _standingaxis (+ _returnvalue_2 _groundsensitivity))) _array))
          (if (not _returnvalue_6)
            (set `self.IsOnGround` false)
            (else
              (bind _returnvalue_7 (`KismetMathLibrary.Normal` (`.ImpactNormal` (`GameplayStatics.BreakHitResult` _outhit_2))))
              (set `self.GroundAxis` _returnvalue_7)
              (set `self.IsOnGround` (<= (`/Game/Asset/DirectionalGravity/Blueprints/Helpers/BP_MathHelpers.AngleBetween` _returnvalue_7 (`self.StandingAxis`)) (`self.GroundMaxSlopeAngle`))))))))))

(fn `CorrectMovementDirection`
  (params (Direction :type "Vector Structure") (Normal :type "Vector Structure"))
  (returns (Result :type "Vector Structure"))
  (return (`KismetMathLibrary.Normal` (- Direction (* Normal (`KismetMathLibrary.Dot_VectorVector` Direction Normal))))))

(fn `ShowVelosity`
  (locals (time_new :type "Float (double-precision)") (time :type "Float (double-precision)") (`end pos` :type "Vector Structure") (`start pos` :type "Vector Structure"))
  (set `local.time_new` (`KismetSystemLibrary.GetGameTimeInSeconds`))
  (set `local.end pos` (`SceneComponent.K2_GetComponentLocation` (`self.WalkCollision`)))
  (if (> (- (`local.time_new`) (`local.time`)) 1.0)
    (`KismetSystemLibrary.PrintString` (`KismetStringLibrary.Concat_StrStr` "Velosity: " (`KismetStringLibrary.Conv_DoubleToString` (/ (`KismetMathLibrary.Vector_Distance` (`local.start pos`) (`local.end pos`)) (- (`local.time_new`) (`local.time`))))) true true (struct :`G` 0.66 :`B` 1.0 :`A` 1.0) 1.0)
    (bind _output_get (set `local.time` (`KismetSystemLibrary.GetGameTimeInSeconds`)))
    (set `local.time_new` _output_get)
    (set `local.start pos` (`SceneComponent.K2_GetComponentLocation` (`self.WalkCollision`)))))

(fn `UpdateStanding`
  (locals (OldForward :type "Vector Structure"))
  (bind _walkcollision (`self.WalkCollision`))
  (bind _lookuplimit (`self.LookUpLimit`))
  (set `local.OldForward` (`SceneComponent.GetForwardVector` (`self.CameraHolder`)))
  ;[1 1 1] Rotate character
  (`PrimitiveComponent.SetConstraintMode` _walkcollision "None")
  (`SceneComponent.K2_SetWorldRotation` _walkcollision (`/Game/Asset/DirectionalGravity/Blueprints/Helpers/BP_MathHelpers.RotatorBetween` (`KismetMathLibrary.MakeVector` 0.0 0.0 1.0) (`self.StandingAxis`)) false false)
  (`PrimitiveComponent.SetConstraintMode` _walkcollision "Default")
  (if (`self.PreserveLookingDirection`)
    ;[1 1 1] Rotate camera to preserve looking direction
    (`SceneComponent.K2_SetRelativeRotation` (`self.CameraHolder`) (`KismetMathLibrary.MakeRotator` 0.0 (`KismetMathLibrary.ClampAngle` (.pitch (`KismetMathLibrary.InverseTransformRotation` (`SceneComponent.K2_GetComponentToWorld` (`self.WalkCollision`)) (`KismetMathLibrary.Conv_VectorToRotator` (`local.OldForward`)))) (- 0.0 _lookuplimit) _lookuplimit) (.yaw (`KismetMathLibrary.InverseTransformRotation` (`SceneComponent.K2_GetComponentToWorld` (`self.WalkCollision`)) (`KismetMathLibrary.Conv_VectorToRotator` (`local.OldForward`))))) false false)))

(fn `UserConstructionScript`
  (`SceneComponent.SetHiddenInGame` (`self.WalkCollision`) (not (`self.Debug`)) false)
  (`SceneComponent.SetHiddenInGame` (`self.SideCollision`) (not (`self.Debug`)) false))