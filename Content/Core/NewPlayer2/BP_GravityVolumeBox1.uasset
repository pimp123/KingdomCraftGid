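; BP_GravityVolumeBox1 is a gravity volume actor that updates the gravity of a character entering it.
; When its Sphere component begins overlapping a BP_GravityCharacter, it passes the actor's location to that character's UpdatePlanetGravityNew, despite the Box in the asset name.
; A separate SetGravity function, not called within this Blueprint, applies a given gravity direction to the movement component of every GravityCharacter in the world.
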(event `self.Sphere.OnComponentBeginOverlap`
  (params (OverlappedComponent :type "PrimitiveComponent Object Reference") (OtherActor :type "Actor Object Reference") (OtherComp :type "PrimitiveComponent Object Reference") (OtherBodyIndex :type Integer) (bFromSweep :type Boolean) (SweepResult :type "HitResult Structure (by ref)"))
  (bind _asbp_gravity_character (cast `/DirGravity/Character/BP_GravityCharacter` OtherActor))
  (`/DirGravity/Character/BP_GravityCharacter.UpdatePlanetGravityNew` _asbp_gravity_character (`self.K2_GetActorLocation`)))

(fn `SetGravity`
  (params (NewGravityDirection :type "Vector Structure"))
  (bind _outactors (`GameplayStatics.GetAllActorsOfClass` "/Script/DirGravity.GravityCharacter"))
  (for _array_element _outactors
    (`GravityMovementComponent.SetGravityDir` (`GravityCharacter.GetGravityMovementComponent` _array_element) NewGravityDirection)))

(fn `UserConstructionScript`
  (`parent.UserConstructionScript`))